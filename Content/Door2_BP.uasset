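; Door Blueprint that swings open and closed on alternate interactions.
; The Interaction event calls UseDoor, where a FlipFlop plays or reverses a timeline.
; The timeline's float track drives a yaw offset combined with the rotation cached at BeginPlay, and its Sound Timing event track plays a door lock cue at the actor's location.
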(event `self.ReceiveBeginPlay`
  (set `self.Initial Rotation` (`self.K2_GetActorRotation`)))

(event `UseDoor`
  (`/Engine/EditorBlueprintResources/StandardMacros.FlipFlop`
    (:`A`
      (bind (_direction `_새_트랙_0`) (`Timeline|타임라인_0` :!label _label)
        (:`Update`
          (`self.K2_SetActorRotation` (`KismetMathLibrary.ComposeRotators` (`KismetMathLibrary.MakeRotator` 0.0 0.0 `_새_트랙_0`) (`self.Initial Rotation`))))
        (:`Sound Timing`
          (`GameplayStatics.PlaySoundAtLocation` "/Game/StarterContent/Audio/door-lock_Cue.door-lock_Cue" (`self.K2_GetActorLocation`)))))
    (:`B`
      (goto _label :!via `Reverse`))))

(event `/Game/BPI.Interaction`
  (`self.UseDoor`))

(fn `UserConstructionScript`)