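; Trigger box Blueprint that operates a referenced door when an actor tagged "key1" enters or leaves its volume.
; Both the begin and end overlap events of the Box component check the tag, cast the Door3 reference to Door3_BP and call UseDoor.
; The same call serves entry and exit, so any open or close logic is left to the door.
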(event `self.Box.OnComponentBeginOverlap`
  (params (OverlappedComponent :type "PrimitiveComponent Object Reference") (OtherActor :type "Actor Object Reference") (OtherComp :type "PrimitiveComponent Object Reference") (OtherBodyIndex :type Integer) (bFromSweep :type Boolean) (SweepResult :type "HitResult Structure (by ref)"))
  (if (`self.ActorHasTag` OtherActor "key1")
    (bind _asdoor_3_bp (cast `/Game/Door3_BP` (`self.Door3`)))
    (`/Game/Door3_BP.UseDoor` _asdoor_3_bp)))

(event `self.Box.OnComponentEndOverlap`
  (params (OverlappedComponent :type "PrimitiveComponent Object Reference") (OtherActor :type "Actor Object Reference") (OtherComp :type "PrimitiveComponent Object Reference") (OtherBodyIndex :type Integer))
  (if (`self.ActorHasTag` OtherActor "key1")
    (bind _asdoor_3_bp (cast `/Game/Door3_BP` (`self.Door3`)))
    (`/Game/Door3_BP.UseDoor` _asdoor_3_bp)))

(fn `UserConstructionScript`)